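; Player component for a stratagem system, where directional input combinations arm an ability actor to spawn at the owner's transform.
; The open action shows the combination HUD, adds a mapping context and resets equipped stratagems, removing both HUD and context on release.
; Directions become data assets that every equipped stratagem checks, and a success event stores the ability for the activate action.
; Init gets controller and HUD references from the owner through message calls.
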(event Custom|E_StratagemSuccessful
  (params (SuccessfulStrategem :type PDA%20Stratagem%20BASE%20Object%20Reference%20%28by%20ref%29))
  ;[0.9572 0 1 0.5] E_StrategemSuccessful
  ;;[0 0.7331 1 0.5] Sets ActiveStrategem to the sucessful strategem
  (Variables|EngineCalc|SetActiveStratagem (Variables|/Game/StratagemSystem/Blueprints/DataAssets/StratagemAbilities/PDA_Stratagem_BASE.PDA_Stratagem_BASE_C|GetAbility SuccessfulStrategem)))

(event Input|EnhancedActionEvents|EnhancedInputActionIA_ActivateStratagem
  (params (ActionValue :type Boolean) (ElapsedSeconds :type Float%20%28double-precision%29) (TriggeredSeconds :type Float%20%28double-precision%29) (InputAction :type Input%20Action%20Object%20Reference :default "/Game/StratagemSystem/Inputs/Actions/IA_ActivateStratagem.IA_ActivateStratagem"))
  ;[1 0.5112 0 0.5] IA_ActivateStrategem
  ;;[0 0 0 0.5] Gets the active strategem and Spawns it
  (bind _activestratagem (Variables|EngineCalc|GetActiveStratagem)
    (:then
      (bind _returnvalue (Game|SpawnActorfromClass _activestratagem (Transformation|GetActorTransform (Components|GetOwner)) "Undefined" "MultiplyWithRoot" 0 0))
      (Development|PrintString (Utilities|GetDisplayName _returnvalue))
      ;;[0 0.9371 1 0.5] Sets ActiveStrategem to null
      (Variables|EngineCalc|SetActiveStratagem 0))
    (:else)))

(event Input|EnhancedActionEvents|EnhancedInputActionIA_DirectionalInputs
  (params (ActionValue :type Vector%202D%20Structure) (ElapsedSeconds :type Float%20%28double-precision%29) (TriggeredSeconds :type Float%20%28double-precision%29) (InputAction :type Input%20Action%20Object%20Reference :default "/Game/StratagemSystem/Inputs/Actions/IA_DirectionalInputs.IA_DirectionalInputs"))
  ;[1 0.4263 0 0.5] IA_DirectionalInputs
  ;;[0 0 0 0.5] Translates input to strategem input and Process the Input
  (bind _stratageminput (CallFunction|TranslateInputtoStratagemInput ActionValue))
  (CallFunction|ProcessInput _stratageminput))

(event Input|EnhancedActionEvents|EnhancedInputActionIA_OpenStratagem
  (params (ActionValue :type Boolean) (ElapsedSeconds :type Float%20%28double-precision%29) (TriggeredSeconds :type Float%20%28double-precision%29) (InputAction :type Input%20Action%20Object%20Reference :default "/Game/StratagemSystem/Inputs/Actions/IA_OpenStratagem.IA_OpenStratagem"))
  (bind _returnvalue (PlayerController|LocalPlayerSubsystems|GetEnhancedInputLocalPlayerSubsystem))
  (bind _hudwidgetref (Variables|Helpers|GetHudWidgetRef))
  ;[1 0.4735 0 0.5] IA_OpenStrategem
  (:Started
    ;;[0 0 0 0.5] Changes visibility of strategems combination ui
    (Default|SetStratagemsCombinationVisibility _hudwidgetref true)
    ;;[0 0 0 0.5] Adds a mapping context and Initialize the equipped strategems
    (Input|AddMappingContext _returnvalue "/Game/StratagemSystem/Inputs/IMC_StratagemControls.IMC_StratagemControls" 0 "(bIgnoreAllPressedKeysUntilRelease=True,bForceImmediately=False,bNotifyUserSettings=False)")
    (CallFunction|InitStratagems))
  (:Canceled
    (Default|SetStratagemsCombinationVisibility _hudwidgetref false :!label _label)
    ;;[0 0 0 0.5] Removes the mappong context
    (Input|RemoveMappingContext _returnvalue "/Game/StratagemSystem/Inputs/IMC_StratagemControls.IMC_StratagemControls" "(bIgnoreAllPressedKeysUntilRelease=True,bForceImmediately=False,bNotifyUserSettings=False)"))
  (:Completed
    (goto _label)))

(event EventBeginPlay)

(fn TranslateInputtoStratagemInput
  (params (ActionValue :type Vector%202D%20Structure))
  ;[0 0 0 0.5] Receives and Sends an Action Value to InputTranslation macro identifies the direction (Up/Down/Left/Right)
  (Utilities|InputTranslation ActionValue
    (:Up
      (Development|PrintString "UP")
      ;[0 0.8155 1 0.5] Sets the corresponding stratagem input data asset
      (LocalVariables|SetLocalStratagemInput "/Game/StratagemSystem/Blueprints/DataAssets/StratagemInputs/DA_Up.DA_Up"))
    (:Down
      (Development|PrintString "DOWN")
      (LocalVariables|SetLocalStratagemInput "/Game/StratagemSystem/Blueprints/DataAssets/StratagemInputs/DA_Down.DA_Down"))
    (:Left
      (Development|PrintString "LEFT")
      (LocalVariables|SetLocalStratagemInput "/Game/StratagemSystem/Blueprints/DataAssets/StratagemInputs/DA_Left.DA_Left"))
    (:Right
      (Development|PrintString "RIGHT")
      (LocalVariables|SetLocalStratagemInput "/Game/StratagemSystem/Blueprints/DataAssets/StratagemInputs/DA_Right.DA_Right")))
  ;[0 0 0 0.5] Returns the stratagem input data asset
  (return (LocalVariables|GetLocalStratagemInput)))

(fn ProcessInput
  (params (StrategemInput :type PDA%20Stratagem%20Input%20Object%20Reference))
  ;[0 0 0 0.5] For each valid equipped stratagem, Calls ProcessNewStrategemInput to verify and Process the new input based on the player input
  (for _array_element (Variables|Config|GetEquippedStratagems)
    (Utilities|IsValid _array_element
      (:Is%20Valid
        (Default|ProcessNewStrategemInput _array_element StrategemInput))
      (:Is%20Not%20Valid
        (CallFunction|DDebugLog "Stratagem" "not valid" "(R=1.000000,G=0.000000,B=0.000017,A=1.000000)" 1e+01))))
  (return))

(fn InitStratagems
  ;[0 0.8409 1 0.5] Sets ActiveStratagem to null
  (Variables|EngineCalc|SetActiveStratagem 0)
  ;[0 0 0 0.5] For each valid equipped stratagem, it initializes and bind the StratagemSuccessful to a custom event
  (for _array_element (Variables|Config|GetEquippedStratagems)
    (Utilities|IsValid _array_element
      (:Is%20Valid
        (Default|Init _array_element)
        (EventDispatchers|BindEventtoStratagemSuccessful _array_element (EventDispatchers|CreateEvent :!event Custom|E_StratagemSuccessful)))
      (:Is%20Not%20Valid
        (CallFunction|DDebugLog "Stratagem" "not valid" "(R=1.000000,G=0.000000,B=0.000017,A=1.000000)" 1e+01))))
  (Default|CallStratagemStartInput)
  (return))

(fn Init
  ;[0 0 0 0.5] Initialize the component of the Stratagem System
  ;;[0 0.8853 1 0.5] Gets player controller from owner and sets to PlayerControllerRef
  (bind _playercontroller (Class|BPIGetPlayerController|GetPlayerController(Message) (Components|GetOwner)))
  (Variables|Helpers|SetPlayerControllerRef _playercontroller)
  ;;[0 0.8853 1 0.5] Gets hud widget from owner and sets to HudWidgetRef
  (bind _hudwidget (Class|BPIGetHudWidget|GetHudWidget(Message) (Components|GetOwner)))
  (bind _output_get (Variables|Helpers|SetHudWidgetRef _hudwidget))
  ;;[0 0 0 0.5] Constructs ui combination of the stratagems
  (Default|ConstructStratagems _output_get (Variables|Config|GetEquippedStratagems)))

(fn DDebugLog
  (params (ObjectName :type String) (Result :type String) (Color :type Linear%20Color%20Structure :default "(R=0.000000,G=0.981388,B=1.000000,A=1.000000)") (Duration :type Float%20%28single-precision%29))
  (Development|PrintString (Utilities|String|Append ObjectName " " Result) true true Color Duration))