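; BP_CharacterBase is the base character of the Stratagem System, holding simple health and death state.
; On BeginPlay it calls ResetStats, which restores current health to maximum and clears the dead flag.
; GetDamage subtracts incoming damage from current health, clamped at zero, but does not set the dead flag.
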(event EventBeginPlay
  (CallFunction|ResetStats))

(event Collision|EventActorBeginOverlap
  (params (OtherActor :type Actor%20Object%20Reference)))

(event EventTick
  (params (DeltaSeconds :type Float%20%28single-precision%29)))

(fn ConstructionScript)

(fn ResetStats
  (Variables|EngineCalc|SetCurrentHealth (Variables|Stats|GetMaxHealth))
  (Variables|EngineCalc|SetIsDead false))

(fn GetDamage
  (params (Damage :type Float%20%28double-precision%29))
  (Variables|EngineCalc|SetCurrentHealth (Math|Float|Max(Float) (- (Variables|EngineCalc|GetCurrentHealth) Damage) 0.0))
  (return))