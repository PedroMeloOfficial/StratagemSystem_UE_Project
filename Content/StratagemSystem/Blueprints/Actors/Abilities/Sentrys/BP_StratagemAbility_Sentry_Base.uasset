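; Base sentry stratagem ability: a turret that shoots at characters it sees, skipping those that implement BPI_GetPlayerController.
; Init pulls the sentry data asset from the stratagem data and sets the PawnSensing sight radius from its range.
; Each OnSeePawn event turns the whole actor toward the target and fires one debug-drawn hitscan trace within a random spread cone.
; Whatever the trace hits receives the damage message; a box-trace target check is left unconnected.
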(event OnSeePawn(PawnSensing)
  (params (Pawn :type Pawn%20Object%20Reference))
  (bind _asbp_character_base (Utilities|Casting|CastToBP_CharacterBase Pawn))
  (if (not (Utilities|DoesObjectImplementInterface _asbp_character_base "/Game/StratagemSystem/Blueprints/Interfaces/BPI_GetPlayerController.BPI_GetPlayerController_C"))
    (Transformation|SetActorRotation (Math|Rotator|FindLookatRotation (Transformation|GetActorLocation) (Transformation|GetActorLocation _asbp_character_base)))
    (bind _hitactor (CallFunction|FireHitScan))
    (Class|BPIDamageable|GetDamage(Message) _hitactor _hitactor (Variables|/Game/StratagemSystem/Blueprints/DataAssets/StratagemAbilities/PDA_Stratagem_BASE.PDA_Stratagem_BASE_C|GetDamage/Heal (Variables|EngineCalc|GetPDA%20Stratagem%20Sentry)))))

(event EventBeginPlay
  (|CallParentFunction) ; This node is disabled and will not be called.\nDrag off pins to build functionality.
)

(event Collision|EventActorBeginOverlap
  (params (OtherActor :type Actor%20Object%20Reference))
  (|CallParentFunction 0))

(event EventTick
  (params (DeltaSeconds :type Float%20%28single-precision%29))
  (|CallParentFunction DeltaSeconds))

(event EventInit
  (|CallParentFunction)
  (bind _pda_stratagemsentry (Class|BPIGetPDAStratagem|GetStratagemSentry(Message) (Variables|Default|GetStratagemDataAsset)))
  (Variables|EngineCalc|SetPDA%20Stratagem%20Sentry _pda_stratagemsentry)
  (Variables|/Script/AIModule.PawnSensingComponent|SetSightRadius (Variables|Default|GetPawnSensing) (Variables|/Game/StratagemSystem/Blueprints/DataAssets/StratagemAbilities/Sentrys/PDA_Stratagem_Sentrys.PDA_Stratagem_Sentrys_C|GetRange (Variables|EngineCalc|GetPDA%20Stratagem%20Sentry))))

(fn ConstructionScript
  (|CallParentFunction))

(fn FireHitScan
  (bind _pda_stratagem_sentry (Variables|EngineCalc|GetPDA%20Stratagem%20Sentry))
  (bind _turrettest (Variables|Default|GetturretTest))
  (bind _returnvalue (Transformation|GetSocketLocation _turrettest "Muzzle"))
  (bind _outhit (Collision|LineTraceByChannel _returnvalue (+ _returnvalue (* (Math|Random|RandomUnitVectorinConeinDegrees (Math|Vector|GetForwardVector (Transformation|GetSocketRotation _turrettest "Muzzle")) (Variables|/Game/StratagemSystem/Blueprints/DataAssets/StratagemAbilities/Sentrys/PDA_Stratagem_Sentrys.PDA_Stratagem_Sentrys_C|GetBulletSpread _pda_stratagem_sentry)) (Variables|/Game/StratagemSystem/Blueprints/DataAssets/StratagemAbilities/Sentrys/PDA_Stratagem_Sentrys.PDA_Stratagem_Sentrys_C|GetRange _pda_stratagem_sentry))) "TraceTypeQuery2" false 0 "ForOneFrame"))
  (return (.HitActor (Collision|BreakHitResult _outhit)) (.ImpactPoint (Collision|BreakHitResult _outhit))))