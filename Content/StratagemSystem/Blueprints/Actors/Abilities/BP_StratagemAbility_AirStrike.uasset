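; BP_StratagemAbility_AirStrike is the air strike ability actor for the stratagem system, dealing area damage to characters.
; On BeginPlay it waits a short delay, then sends a damage message to every character overlapping its sphere.
; A hit event on the sphere also sends the same damage message to whatever actor it collides with.
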(event OnComponentHit(Sphere)
  (params (HitComponent :type Primitive%20Component%20Object%20Reference) (OtherActor :type Actor%20Object%20Reference) (OtherComp :type Primitive%20Component%20Object%20Reference) (NormalImpulse :type Vector :default "0, 0, 0") (Hit :type Hit%20Result%20Structure%20%28by%20ref%29))
  (Class|BPIDamageable|GetDamage(Message) OtherActor OtherActor 1e+02))

(event EventBeginPlay
  (|CallParentFunction)
  (Utilities|FlowControl|Delay 2.5)
  (for _array_element (Collision|GetOverlappingActors (Variables|Default|GetSphere) "/Game/StratagemSystem/Blueprints/Actors/Characters/BP_CharacterBase.BP_CharacterBase_C" :!class /Script/Engine.PrimitiveComponent)
    (Class|BPIDamageable|GetDamage(Message) _array_element _array_element 1e+02)))

(event Collision|EventActorBeginOverlap
  (params (OtherActor :type Actor%20Object%20Reference))
  (|CallParentFunction OtherActor))

(event EventTick
  (params (DeltaSeconds :type Float%20%28single-precision%29))
  (|CallParentFunction DeltaSeconds))

(fn ConstructionScript
  (|CallParentFunction))