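; BP_StratagemAbility_MachineSentry is a stratagem ability actor, named as a machine sentry, that so far holds only placeholder logic.
; On BeginPlay it calls the parent, then runs a debug-drawn Camera-channel line trace using the static mesh's forward vector as the start position, with no end wired.
; The trace result is unused, Tick and overlap events are disabled, and the construction script only calls its parent.
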(event EventBeginPlay
  (|CallParentFunction)
  (Collision|LineTraceByChannel (Math|Vector|GetForwardVector (Variables|Default|GetStaticMesh)) "0, 0, 0" "TraceTypeQuery2" false 0 "ForDuration"))

(event Collision|EventActorBeginOverlap
  (params (OtherActor :type Actor%20Object%20Reference))
  (|CallParentFunction OtherActor) ; This node is disabled and will not be called.\nDrag off pins to build functionality.
)

(event EventTick
  (params (DeltaSeconds :type Float%20%28single-precision%29))
  (|CallParentFunction DeltaSeconds) ; This node is disabled and will not be called.\nDrag off pins to build functionality.
)

(fn ConstructionScript
  (|CallParentFunction))