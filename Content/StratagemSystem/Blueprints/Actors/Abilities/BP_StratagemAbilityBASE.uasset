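; Base actor for stratagem abilities: a lobbed projectile that triggers a delayed effect defined by its StratagemDataAsset.
; On BeginPlay it launches forward and upward, assigns the asset's particle template, then activates it after the asset's delay.
; Particle spawn events play the asset's sound at their location, and the actor destroys itself when the system finishes.
; A helper prints debug messages for an invalid asset and for destruction.
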(event OnSystemFinished(ParticleSystem)
  (params (PSystem :type Particle%20System%20Component%20Object%20Reference))
  (Actor|DestroyActor)
  (CallFunction|DDebugLog self "destroyed" "" "(R=0.000000,G=0.892583,B=1.000000,A=1.000000)" 3.0))

(event OnParticleSpawn(ParticleSystem)
  (params (EventName :type Name :default "None") (EmitterTime :type Float%20%28single-precision%29) (Location :type Vector :default "0, 0, 0") (Velocity :type Vector :default "0, 0, 0"))
  (Audio|PlaySoundatLocation (Variables|/Game/StratagemSystem/Blueprints/DataAssets/StratagemAbilities/PDA_Stratagem.PDA_Stratagem_C|GetSFX%20Sound (Variables|Default|GetStratagemDataAsset)) Location "0, 0, 0" 1.0 1.0 0.0 0 0 0 0))

(event EventBeginPlay
  (bind _stratagemdataasset (Variables|Default|GetStratagemDataAsset)
    (:then
      (Game|Components|ProjectileMovement|SetVelocityinLocalSpace (Variables|Default|GetProjectileMovement) "700.000000,0.000000,500.000000")
      (Effects|Components|ParticleSystem|SetTemplate (Variables|Default|GetParticleSystem) (Variables|/Game/StratagemSystem/Blueprints/DataAssets/StratagemAbilities/PDA_Stratagem.PDA_Stratagem_C|GetVFX%20Particle (Variables|Default|GetStratagemDataAsset)))
      (Utilities|FlowControl|Delay (Variables|/Game/StratagemSystem/Blueprints/DataAssets/StratagemAbilities/PDA_Stratagem.PDA_Stratagem_C|GetDelayToExec (Variables|Default|GetStratagemDataAsset)))
      (Components|Activation|Activate (Variables|Default|GetParticleSystem) false))
    (:else
      (CallFunction|DDebugLog _stratagemdataasset "not valid" "StratagemDataAsset" "(R=1.000000,G=0.000000,B=0.000017,A=1.000000)" 1e+01))))

(event EventTick
  (params (DeltaSeconds :type Float%20%28single-precision%29)))

(fn ConstructionScript)

(fn DDebugLog
  (params (Object :type Object%20Object%20Reference) (Result :type String) (ObjectName :type String) (Color :type Linear%20Color%20Structure :default "(R=0.000000,G=0.892583,B=1.000000,A=1.000000)") (Duration :type Float%20%28single-precision%29))
  (Development|PrintString (Utilities|String|Append (Utilities|GetDisplayName Object) " " ObjectName " " Result) true true Color Duration))