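; Player component for directional-combination stratagems, which unlock an ability to spawn.
; Holding the open input shows the HUD combination display, adds a control mapping context and re-initializes the equipped stratagems.
; Directional input becomes Up/Down/Left/Right data assets fed to every equipped stratagem.
; A stratagem's success event stores its ability class, which the activate input spawns at the owner's transform and then clears.
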(event Custom|E_StrategemSuccessful
  (params (SuccessfulStrategem :type PDA%20Strategem%20Object%20Reference))
  ;[1 0.6281 0.2094 0.5] E_StrategemSuccessful
  ;;[0 0.7331 1 0.5] Sets ActiveStrategem to the sucessful strategem
  (Variables|Default|SetActiveStrategem (Variables|/Game/StrategemSystem/Blueprints/DataAssets/Strategems/PDA_Strategem.PDA_Strategem_C|GetAbility SuccessfulStrategem)))

(event Input|EnhancedActionEvents|EnhancedInputActionIA_ActivateStrategem
  (params (ActionValue :type Boolean) (ElapsedSeconds :type Float%20%28double-precision%29) (TriggeredSeconds :type Float%20%28double-precision%29) (InputAction :type Input%20Action%20Object%20Reference :default "/Game/StrategemSystem/Inputs/Actions/IA_ActivateStrategem.IA_ActivateStrategem"))
  ;[1 0.5112 0 0.5] IA_ActivateStrategem
  (:Triggered
    ;;[0 0 0 0.5] Gets the active strategem and Spawns it
    (bind _activestrategem (Variables|Default|GetActiveStrategem)
      (:then
        (bind _returnvalue (Game|SpawnActorfromClass _activestrategem (Transformation|GetActorTransform (Components|GetOwner)) "Undefined" "MultiplyWithRoot" 0 0))
        (Development|PrintString (Utilities|GetDisplayName _returnvalue))
        ;;[0 0.9371 1 0.5] Sets ActiveStrategem to null
        (Variables|Default|SetActiveStrategem 0))
      (:else))))

(event Input|EnhancedActionEvents|EnhancedInputActionIA_DirectionalInputs
  (params (ActionValue :type Vector%202D%20Structure) (ElapsedSeconds :type Float%20%28double-precision%29) (TriggeredSeconds :type Float%20%28double-precision%29) (InputAction :type Input%20Action%20Object%20Reference :default "/Game/StrategemSystem/Inputs/Actions/IA_DirectionalInputs.IA_DirectionalInputs"))
  ;[1 0.4263 0 0.5] IA_DirectionalInputs
  ;;[0 0 0 0.5] Translates input to strategem input and Process the Input
  (bind _strategeminput (CallFunction|TranslateInputtoStrategemInput ActionValue))
  (CallFunction|ProcessInput _strategeminput))

(event Input|EnhancedActionEvents|EnhancedInputActionIA_OpenStrategem
  (params (ActionValue :type Boolean) (ElapsedSeconds :type Float%20%28double-precision%29) (TriggeredSeconds :type Float%20%28double-precision%29) (InputAction :type Input%20Action%20Object%20Reference :default "/Game/StrategemSystem/Inputs/Actions/IA_OpenStrategem.IA_OpenStrategem"))
  (bind _returnvalue (PlayerController|LocalPlayerSubsystems|GetEnhancedInputLocalPlayerSubsystem))
  (bind _hudwidgetref (Variables|Default|GetHudWidgetRef))
  ;[1 0.4735 0 0.5] IA_OpenStrategem
  (:Started
    (Default|SetStrategemsCombinationVisibility _hudwidgetref true)
    ;;[0 0 0 0.5] Adds a mapping context and Initialize the equipped strategems
    (Input|AddMappingContext _returnvalue "/Game/StrategemSystem/Inputs/IMC_StrategemControls.IMC_StrategemControls" 0 "(bIgnoreAllPressedKeysUntilRelease=True,bForceImmediately=False,bNotifyUserSettings=False)")
    (CallFunction|InitStrategems))
  (:Canceled
    (Default|SetStrategemsCombinationVisibility _hudwidgetref false :!label _label)
    ;;[0 0 0 0.5] Removes the mappong context
    (Input|RemoveMappingContext _returnvalue "/Game/StrategemSystem/Inputs/IMC_StrategemControls.IMC_StrategemControls" "(bIgnoreAllPressedKeysUntilRelease=True,bForceImmediately=False,bNotifyUserSettings=False)"))
  (:Completed
    (goto _label)))

(event EventBeginPlay
  ;[0 0 0 0.5] BeginPlay
  ;;[0 0.8853 1 0.5] Gets player controller from owner and sets to PlayerControllerRef
  (bind _playercontroller (Class|BPIGetPlayerController|GetPlayerController(Message) (Components|GetOwner)))
  (Variables|Default|SetPlayerControllerRef _playercontroller)
  ;;[0 0.8853 1 0.5] Gets hud widget from owner and sets to HudWidgetRef
  (bind _hudwidget (Class|BPIGetHudWidget|GetHudWidget(Message) (Components|GetOwner)))
  (Variables|Default|SetHudWidgetRef _hudwidget))

(fn TranslateInputtoStrategemInput
  (params (ActionValue :type Vector%202D%20Structure))
  ;[0 0 0 0.5] Receives and Sends an Action Value to InputTranslation macro identifies the direction (Up/Down/Left/Right)
  (Utilities|InputTranslation ActionValue
    (:Up
      (Development|PrintString "UP")
      ;[0 0.8155 1 0.5] Sets the corresponding stratagem input data asset
      (LocalVariables|SetLocalStrategemInput "/Game/StrategemSystem/Blueprints/DataAssets/DA_Up.DA_Up"))
    (:Down
      (Development|PrintString "DOWN")
      (LocalVariables|SetLocalStrategemInput "/Game/StrategemSystem/Blueprints/DataAssets/DA_Down.DA_Down"))
    (:Left
      (Development|PrintString "LEFT")
      (LocalVariables|SetLocalStrategemInput "/Game/StrategemSystem/Blueprints/DataAssets/DA_Left.DA_Left"))
    (:Right
      (Development|PrintString "RIGHT")
      (LocalVariables|SetLocalStrategemInput "/Game/StrategemSystem/Blueprints/DataAssets/DA_Right.DA_Right")))
  ;[0 0 0 0.5] Returns the stratagem input data asset
  (return (LocalVariables|GetLocalStrategemInput)))

(fn ProcessInput
  (params (StrategemInput :type PDA%20Strategem%20Input%20Object%20Reference))
  ;[0 0 0 0.5] For each equipped strategem, Calls ProcessNewStrategemInput to verify and Process the new input based on the player input
  (for _array_element (Variables|Default|GetEquippedStrategems)
    (Default|ProcessNewStrategemInput _array_element StrategemInput))
  (return))

(fn InitStrategems
  ;[0 0.8409 1 0.5] Sets ActiveStrategem to null
  (Variables|Default|SetActiveStrategem 0)
  ;[0 0 0 0.5] For each equipped strategem, it initializes and bind the StrategemSuccessful to a custom event
  (for _array_element (Variables|Default|GetEquippedStrategems)
    (Default|Init _array_element)
    (EventDispatchers|BindEventtoStrategemSuccessful _array_element (EventDispatchers|CreateEvent :!event Custom|E_StrategemSuccessful)))
  (Default|CallStrategemStartInput)
  (return))