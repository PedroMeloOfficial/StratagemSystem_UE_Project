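; Base actor for Strategem abilities: a launched projectile that plays a configurable particle effect and sound after a delay.
; On BeginPlay it sets a forward-and-up local velocity, assigns the VFX template, then activates the particle system once the delay elapses.
; The sound plays at the location reported by each particle spawn event.
; When the particle system finishes, the actor destroys itself and prints a deletion message.
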(event OnSystemFinished(ParticleSystem)
  (params (PSystem :type Particle%20System%20Component%20Object%20Reference))
  (Actor|DestroyActor)
  (Development|PrintString (Utilities|String|Append (Utilities|GetDisplayName self) " deleted") true true "(R=0.000000,G=0.660000,B=1.000000,A=1.000000)" 5.0))

(event OnParticleSpawn(ParticleSystem)
  (params (EventName :type Name :default "None") (EmitterTime :type Float%20%28single-precision%29) (Location :type Vector :default "0, 0, 0") (Velocity :type Vector :default "0, 0, 0"))
  (Audio|PlaySoundatLocation (Variables|Default|GetSFX%20Sound) Location "0, 0, 0" 1.0 1.0 0.0 0 0 0 0))

(event EventBeginPlay
  (Game|Components|ProjectileMovement|SetVelocityinLocalSpace (Variables|Default|GetProjectileMovement) "700.000000,0.000000,500.000000")
  (Effects|Components|ParticleSystem|SetTemplate (Variables|Default|GetParticleSystem) (Variables|Default|GetVFX%20Particle))
  (Utilities|FlowControl|Delay (Variables|Default|GetDelayDuration))
  (Components|Activation|Activate (Variables|Default|GetParticleSystem) false))

(event Collision|EventActorBeginOverlap
  (params (OtherActor :type Actor%20Object%20Reference)))

(event EventTick
  (params (DeltaSeconds :type Float%20%28single-precision%29)))

(fn ConstructionScript)